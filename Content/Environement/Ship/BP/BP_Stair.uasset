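; BP_Stair is a ship stair Blueprint meant to toggle its Box collision based on the player character's movement speed.
; The Collisionstair event disables the Box's collision at or above a small speed threshold and sets it to query-only below it.
; The setup that caches the player character and starts a looping timer for this check is disconnected.
; BeginPlay is empty, so nothing in this graph starts the toggle.
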(event Custom|Event%20Collision%20stair
  (bind _box (Variables|Default|GetBox))
  (if (>= (Math|Vector|VectorLength (Transformation|GetVelocity (Variables|Default|GetAs%20BP%20Third%20Person%20Character))) 5e+01)
    (Collision|SetCollisionEnabled _box "NoCollision")
    (else
      (Collision|SetCollisionEnabled _box "QueryOnly"))))

(event EventBeginPlay)

(fn ConstructionScript)
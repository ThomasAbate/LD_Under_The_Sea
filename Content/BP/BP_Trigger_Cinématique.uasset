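; BP_Trigger_Cinématique is a trigger that starts a cinematic when the third-person player character enters its collision component.
; On overlap it creates a player for the assigned Level Sequence, plays it, then calls HidienPlayer.
; That event teleports the player character to the Target actor's location and rotation and disables input.
; The graph never re-enables input and has no guard against repeat triggering.
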(event OnComponentBeginOverlap(CollisionComponent)
  (params (OverlappedComponent :type Primitive%20Component%20Object%20Reference) (OtherActor :type Actor%20Object%20Reference) (OtherComp :type Primitive%20Component%20Object%20Reference) (OtherBodyIndex :type Integer) (bFromSweep :type Boolean) (SweepResult :type Hit%20Result%20Structure%20%28by%20ref%29))
  (Utilities|Casting|CastToBP_ThirdPersonCharacter OtherActor)
  (bind _returnvalue (Sequencer|Player|CreateLevelSequencePlayer (Variables|Default|GetLevel%20Sequence)))
  (Sequencer|Player|Play _returnvalue :!class /Script/MovieScene.MovieSceneSequencePlayer)
  (CallFunction|EventHidienPlayer))

(event Custom|Event%20Hidien%20Player
  (bind _returnvalue (Game|GetPlayerController 0))
  (bind _target (Variables|Default|GetTarget))
  (bind _returnvalue_2 (Transformation|GetActorTransform _target))
  (Transformation|Teleport (Game|GetPlayerCharacter 0) (.location _returnvalue_2) (.rotation _returnvalue_2))
  (Input|DisableInput _returnvalue _returnvalue))

(fn ConstructionScript)
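; BP_Door is an interactable door that opens by removing its door component and fading its remaining static mesh.
; Its interaction function destroys SMDoor, then sets StaticMesh to overlap the Visibility and Camera channels.
; It then creates a dynamic material instance on the mesh's first material slot and switches on the Fade_On parameter.
; The event graph has no active logic, and the function has no path to reverse the change.
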(event EventBeginPlay
  (|CallParentFunction) ; This node is disabled and will not be called.\nDrag off pins to build functionality.
)

(event Collision|EventActorBeginOverlap
  (params (OtherActor :type Actor%20Object%20Reference)))

(event EventTick
  (params (DeltaSeconds :type Float%20%28single-precision%29)))

(fn ConstructionScript
  (|CallParentFunction))

(fn InteractionFonction
  (bind _staticmesh (Variables|Default|GetStaticMesh))
  (Components|DestroyComponent (Variables|Default|GetSM_Door))
  (Collision|SetCollisionResponsetoChannel _staticmesh "ECC_Visibility" "ECR_Overlap")
  (Collision|SetCollisionResponsetoChannel _staticmesh "ECC_Camera" "ECR_Overlap")
  (bind _returnvalue (Rendering|Material|CreateDynamicMaterialInstance _staticmesh 0 (Rendering|Material|GetMaterial _staticmesh 0) "None" :!class /Script/Engine.PrimitiveComponent))
  (Rendering|Material|SetScalarParameterValue _returnvalue "Fade_On" 1.0 :!class /Script/Engine.MaterialInstanceDynamic))
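; BP_Produit is an interactable product pickup that adds to the player's collected score.
; Its InteractionFonction casts the player character to BP_ThirdPersonCharacter, increments BenCollected directly on that character's WidgetScore, then destroys the actor.
; The count lives in the score widget, and the event graph holds only disabled default events.
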(event EventBeginPlay
  (|CallParentFunction) ; This node is disabled and will not be called.\nDrag off pins to build functionality.
)

(event Collision|EventActorBeginOverlap
  (params (OtherActor :type Actor%20Object%20Reference)))

(event EventTick
  (params (DeltaSeconds :type Float%20%28single-precision%29)))

(fn ConstructionScript
  (|CallParentFunction))

(fn InteractionFonction
  (bind _asbp_third_person_character (Utilities|Casting|CastToBP_ThirdPersonCharacter (Game|GetPlayerCharacter 0)))
  (bind _result (Math|Integer|IncrementInt (Variables|/Game/ThirdPerson/Blueprints/WBP_Score.WBP_Score_C|GetBen%20Collected (Variables|/Game/ThirdPerson/Blueprints/BP_ThirdPersonCharacter.BP_ThirdPersonCharacter_C|GetWidget%20Score _asbp_third_person_character)))
    (:%20%20
      (Variables|/Game/ThirdPerson/Blueprints/WBP_Score.WBP_Score_C|SetBen%20Collected (Variables|/Game/ThirdPerson/Blueprints/BP_ThirdPersonCharacter.BP_ThirdPersonCharacter_C|GetWidget%20Score _asbp_third_person_character) _result)
      (Actor|DestroyActor))))
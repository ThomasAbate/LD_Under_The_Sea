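; BP_Trap is an interactable trap that slides its SMTrap component once when its interaction function is called.
; InteractionFonction fires the TrapAnimation event, then destroys TriggerBox.
; TrapAnimation plays a timeline whose alpha lerps between two relative locations along X, passing each result to MoveComponentTo while keeping the current rotation.
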(event Custom|Event%20Trap%20Animation
  (bind _sm_trap (Variables|Default|GetSM_Trap))
  (bind _alpha (Timeline|Timeline Play)
    (:Update
      (Components|MoveComponentTo _sm_trap (Math|Vector|Lerp(Vector) "40.000000,0.000000,10.000000" "-70.000000,0.000000,10.000000" _alpha) (Variables|/Script/Engine.SceneComponent|GetRelativeRotation _sm_trap) false false 0.2 false))))

(fn ConstructionScript
  (|CallParentFunction))

(fn InteractionFonction
  (CallFunction|EventTrapAnimation)
  (Components|DestroyComponent (Variables|Default|GetTrigger%20Box)))
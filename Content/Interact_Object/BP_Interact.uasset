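; BP_Interact is an interactable actor that shows an action prompt when the player enters its trigger box and, by default, destroys itself on interaction.
; BeginPlay creates the prompt widget, and the trigger's overlap events add it to or remove it from the viewport.
; Interaction calls InteractionFonction, then sets Activate, which blocks further prompts.
; A looping timer also removes the widget whenever Activate is false.
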(event OnComponentEndOverlap(TriggerBox)
  (params (OverlappedComponent :type Primitive%20Component%20Object%20Reference) (OtherActor :type Actor%20Object%20Reference) (OtherComp :type Primitive%20Component%20Object%20Reference) (OtherBodyIndex :type Integer))
  (if (== (Game|GetPlayerCharacter 0) OtherActor)
    (Widget|RemovefromParent (Variables|Default|GetWidget))))

(event OnComponentBeginOverlap(TriggerBox)
  (params (OverlappedComponent :type Primitive%20Component%20Object%20Reference) (OtherActor :type Actor%20Object%20Reference) (OtherComp :type Primitive%20Component%20Object%20Reference) (OtherBodyIndex :type Integer) (bFromSweep :type Boolean) (SweepResult :type Hit%20Result%20Structure%20%28by%20ref%29))
  (if (== OtherActor (Game|GetPlayerCharacter 0))
    (if (not (Variables|Default|GetActivate))
      (UserInterface|Viewport|AddtoViewport (Variables|Default|GetWidget) 0))))

(event Custom|Event%20Check%20is%20activate
  (if (not (Variables|Default|GetActivate))
    (Widget|RemovefromParent (Variables|Default|GetWidget))))

(event EventBeginPlay
  (bind _returnvalue (UserInterface|CreateWidget "/Game/Interact_Object/Widget/WBP_Action_Widget.WBP_Action_Widget_C" (Game|GetPlayerController 0)))
  (Variables|Default|SetWidget _returnvalue)
  (bind _asbp_third_person_character (Utilities|Casting|CastToBP_ThirdPersonCharacter (Game|GetPlayerCharacter 0)))
  (Variables|Default|SetAs%20BP%20Third%20Person%20Character _asbp_third_person_character)
  (Utilities|Time|SetTimerbyEvent (delegate Custom|Event%20Check%20is%20activate) 0.2 true))

(event EventInteraction
  (if (not (Variables|Default|GetDo%20Once))
    _
    (else
      (Utilities|FlowControl|DoOnce false
        (:Completed
          _))))
  (CallFunction|InteractionFonction)
  (Variables|Default|SetActivate true))

(fn ConstructionScript)

(fn InteractionFonction
  (Actor|DestroyActor))